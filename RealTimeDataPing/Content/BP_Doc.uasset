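; BP_Doc is a test Blueprint that downloads a public Google Sheet as CSV when play begins.
; It requests the same PintUrl twice, each with its own completion callback.
; One callback validates the download through a backup-fallback helper with empty paths, fills the DocTestPing array from the CSV and prints on success.
; The other prints the raw response string to screen.
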(event Custom|CustomEvent_0
  (params (CallbackInfo :type Runtime%20Data%20Table%20Callback%20Info%20Structure))
  (bind _outcsvinfo (Class|RuntimeDataTableObject|ValidateGoogleSheetsDownloadandLoadBackupifNeeded CallbackInfo))
  (bind _successful (Class|RuntimeDataTableObject|UpdateArrayfromCsvInfo (Variables|Default|GetDocTestPing) _outcsvinfo))
  (if _successful
    (Development|PrintString "Well The stuff should be in an array" true true "(R=1.000000,G=0.000000,B=0.000000,A=1.000000)" 1e+01)))

(event Custom|CustomEvent_1
  (params (CallbackInfo :type Runtime%20Data%20Table%20Callback%20Info%20Structure))
  (Development|PrintString (.responseasstring CallbackInfo) true true "(R=1.000000,G=1.000000,B=1.000000,A=1.000000)" 5.0))

(event EventBeginPlay
  (bind _pinturl (Variables|Default|GetPintUrl))
  (Class|RuntimeDataTableObject|BuildGoogleSheetDownloadLinkandGetasCsv :CallOnComplete (delegate Custom|CustomEvent_0) :InSheetURL _pinturl :bSheetIsPublic true)
  (Class|RuntimeDataTableObject|BuildGoogleSheetDownloadLinkandGetasCsv :CallOnComplete (delegate Custom|CustomEvent_1) :InSheetURL _pinturl :bSheetIsPublic true))

(fn ConstructionScript)